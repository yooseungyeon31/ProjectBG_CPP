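; Player controller that routes movement, look, free-look, pose and walk/run input to BP_Player.
; Data tables drive pose transitions, movement lock timers, per-pose pitch limits, camera heights and walk speeds.
; Timelines ease control rotation back within pitch limits and blend spring arm height on pose or movement changes.
; Cached speeds follow move state, with forward or non-forward speed picked by dotting acceleration against facing.
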(event `self.ReceiveTick`
  (params (DeltaSeconds :type "Float (single-precision)")))

(event `self.ReceiveBeginPlay`
  ; save ref 인스턴스 저장하는 노드
  (bind _asbp_player (cast `/Game/Blueprints/Character/BP_Player` (`GameplayStatics.GetPlayerCharacter` 0)))
  (set `self.PlayerRef` _asbp_player)
  (`self.UpdatePitchLimits` "NewEnumerator0")
  ;; 받는쪽에서도 일치하는 함수가 와야한다.
  ;;; 이벤트 디스패처 불러옴, 플레이어가 호출할 때 마다
  (add `/Game/Blueprints/Character/BP_Player.OnMovementStateChanged` (`self.PlayerRef`) (delegate `OnMovementStateChanged`))
  (`self.SetCachedWlalkSpeed`))

(event `OnMovementStateChanged`
  (params (bIsMovingNow :type Boolean))
  (`self.UpdateCameraHeight` bIsMovingNow))

(event `InputAxis|MoveForward`
  (params (AxisValue :type "Float (single-precision)"))
  ; 키보드 인풋
  (if (`self.bIsEnableMove`)
    (`self.UpdateWalkSpeed`)
    (`/Game/Blueprints/Character/BP_Player.Move` (`self.PlayerRef`) true AxisValue)))

(event `InputAxis|Turn`
  (params (AxisValue :type "Float (single-precision)"))
  ; 마우스 인풋
  (`/Game/Blueprints/Character/BP_Player.InputTurn` (`self.PlayerRef`) AxisValue))

(event `InputAxis|MoveRight`
  (params (AxisValue :type "Float (single-precision)"))
  ; 키보드 인풋
  (if (`self.bIsEnableMove`)
    (`self.UpdateWalkSpeed`)
    (`/Game/Blueprints/Character/BP_Player.Move` (`self.PlayerRef`) false AxisValue)))

(event `InputAxis|LookUp`
  (params (AxisValue :type "Float (single-precision)"))
  ; 마우스 인풋
  (if (`self.LimitPitchAngle` AxisValue)
    (`/Game/Blueprints/Character/BP_Player.InputLookUp` (`self.PlayerRef`) AxisValue)))

(event `SetEnableMove`
  ; 데이터 테이블을 사용한 애니메이션 변경  POSE
  (set `self.bIsEnableMove` true))

(event `InputAction|FreeLook`
  (params (Key :type "Key Structure"))
  (bind _playerref (`self.PlayerRef`))
  ; 프리룩 (자유시점)
  ;; alt
  (:`Pressed`
    (`/Game/Blueprints/Character/BP_Player.FreeLook` _playerref true))
  (:`Released`
    (`/Game/Blueprints/Character/BP_Player.FreeLook` _playerref false)))

(event `InputAction|Crouch`
  (params (Key :type "Key Structure"))
  (bind _playerref (`self.PlayerRef`))
  (bind (_transitiontime _topose) (`self.OnTransitionTimer` "NewEnumerator1" (`/Game/Blueprints/Character/BP_Player.CurrentPoseState` _playerref) (`/Game/Blueprints/Character/BP_Player.bIsWeaponEquipped` _playerref)))
  ; 데이터 테이블을 사용한 애니메이션 변경  POSE
  (:`Pressed`
    (`self.UpdatePose` _transitiontime _topose)
    (`self.UpdatePitchLimits` (`/Game/Blueprints/Character/BP_Player.CurrentPoseState` (`self.PlayerRef`)))
    (`self.UpdateCameraHeight` false)
    (`self.UpdateWalkSpeed`)))

(event `InputAction|Prone`
  (params (Key :type "Key Structure"))
  (bind _playerref (`self.PlayerRef`))
  (bind (_transitiontime _topose) (`self.OnTransitionTimer` "NewEnumerator2" (`/Game/Blueprints/Character/BP_Player.CurrentPoseState` _playerref) (`/Game/Blueprints/Character/BP_Player.bIsWeaponEquipped` _playerref)))
  ; 데이터 테이블을 사용한 애니메이션 변경  POSE
  (:`Pressed`
    (`self.UpdatePose` _transitiontime _topose)
    (`self.UpdatePitchLimits` (`/Game/Blueprints/Character/BP_Player.CurrentPoseState` (`self.PlayerRef`)))
    (`self.UpdateCameraHeight` false)
    (`self.UpdateWalkSpeed`)))

(event `InputAction|Jump`
  (params (Key :type "Key Structure"))
  (bind _playerref (`self.PlayerRef`))
  (bind _currentposestate (`/Game/Blueprints/Character/BP_Player.CurrentPoseState` _playerref))
  (bind (_transitiontime _topose) (`self.OnTransitionTimer` "NewEnumerator0" _currentposestate (`/Game/Blueprints/Character/BP_Player.bIsWeaponEquipped` _playerref)))
  ; 데이터 테이블을 사용한 애니메이션 변경  POSE
  (:`Pressed`
    (if (`|EnumEquality` _currentposestate "NewEnumerator0")
      (`Character.Jump` (`self.PlayerRef`))
      (else
        (`self.UpdatePose` _transitiontime _topose)
        (`self.UpdatePitchLimits` (`/Game/Blueprints/Character/BP_Player.CurrentPoseState` (`self.PlayerRef`)))
        (`self.UpdateCameraHeight` false)
        (`self.UpdateWalkSpeed`)))))

(event `InputAction|Walk`
  (params (Key :type "Key Structure"))
  (bind _playerref (`self.PlayerRef`))
  ; MovementState Update
  (:`Pressed`
    (set `/Game/Blueprints/Character/BP_Player.bIsWalkPressed` true _playerref)
    (`/Game/Blueprints/Character/BP_Player.EvaluateMoveState` _playerref :!label _label)
    (`self.SetCachedWlalkSpeed`))
  (:`Released`
    (set `/Game/Blueprints/Character/BP_Player.bIsWalkPressed` false _playerref)
    (goto _label)))

(event `InputAction|Run`
  (params (Key :type "Key Structure"))
  (bind _playerref (`self.PlayerRef`))
  (:`Pressed`
    (set `/Game/Blueprints/Character/BP_Player.bIsRunPressed` true _playerref)
    (`/Game/Blueprints/Character/BP_Player.EvaluateMoveState` _playerref :!label _label_2)
    (`self.SetCachedWlalkSpeed`))
  (:`Released`
    (set `/Game/Blueprints/Character/BP_Player.bIsRunPressed` false _playerref)
    (goto _label_2)))

(event `ChangePitchLimit`
  (params (CurrentRotation :type "Rotator Structure") (TargetRotation :type "Rotator Structure"))
  (bind (_direction _alpha) (`Timeline|TL_ChangePotchLimit` :!via `PlayFromStart`)
    (:`Update`
      (`self.SetControlRotation` (`KismetMathLibrary.RLerp` CurrentRotation TargetRotation _alpha true)))))

(event `ChangedCameraHeight`
  (params (TargetHeight :type "Float (double-precision)") (CurrentHeight :type "Float (double-precision)"))
  (bind _springarm (`/Game/Blueprints/Character/BP_Player.SpringArm` (`self.PlayerRef`)))
  (bind (_socketoffset_x _socketoffset_y) (`KismetMathLibrary.BreakVector` (`SpringArmComponent.SocketOffset` _springarm)))
  (bind (_direction _alpha) (`Timeline|TL_ChangedCameraHeight` :!via `PlayFromStart`)
    (:`Update`
      (set `SpringArmComponent.SocketOffset` (`KismetMathLibrary.MakeVector` _socketoffset_x _socketoffset_y (`KismetMathLibrary.Lerp` CurrentHeight TargetHeight _alpha)) _springarm))))

(fn `IsAcceleratingForwardArc`
  (returns (IsForward :type Boolean))
  (bind _playerref (`self.PlayerRef`))
  (return (>= (`KismetMathLibrary.Dot_VectorVector` (`self.GetActorForwardVector` _playerref) (`KismetMathLibrary.Normal` (`CharacterMovementComponent.GetCurrentAcceleration` (`Character.CharacterMovement` _playerref)))) 0.707)))

(fn `LimitPitchAngle`
  (params (Axis :type "Float (double-precision)"))
  (returns (ReturnValue :type Boolean))
  (bind (_returnvalue_roll _returnvalue_pitch) (`KismetMathLibrary.BreakRotator` (`self.GetControlRotation`)))
  (bind _returnvalue (+ _returnvalue_pitch (* (`local.Axis`) (`self.GetDeprecatedInputPitchScale`))))
  (return (or (> _returnvalue (`self.CachedBottomLimit`)) (< _returnvalue (`self.CachedTopLimit`)))))

(fn `OnTransitionTimer`
  (params (TargetPose :type "/Game/Blueprints/Datas/Enum/E_PoseState Enum" :default "NewEnumerator0") (FromPose :type "/Game/Blueprints/Datas/Enum/E_PoseState Enum" :default "NewEnumerator0") (bIsWeaponEquipped :type Boolean))
  (returns (TransitionTime :type "Float (double-precision)") (ToPose :type "/Game/Blueprints/Datas/Enum/E_PoseState Enum"))
  (locals (ReturnPose :type "/Game/Blueprints/Datas/Enum/E_PoseState Enum" :default "NewEnumerator0"))
  ; DT_ProneTime 데이터테이블을 사용
  (set `local.ReturnPose` (`self.TryGetPoseTransition` TargetPose FromPose))
  (bind _returnvalue (`|GetDataTableRow` "/Game/Blueprints/Datas/DataTable/DT_ProneTime.DT_ProneTime" (`KismetStringLibrary.Conv_StringToName` (`KismetStringLibrary.Concat_StrStr` (`KismetStringLibrary.Conv_BoolToString` bIsWeaponEquipped) "_" (`|GetEnumeratorNameAsString` (`local.FromPose`)) "_" (`|GetEnumeratorNameAsString` (`local.ReturnPose`)))))
    (:`then`
      _)
    (:`RowNotFound`
      _))
  (return (break `/Game/Blueprints/Datas/Struct/ST_ProneTime` _returnvalue) (`local.ReturnPose`)))

(fn `SetCachedWlalkSpeed`
  (locals (RowName :type String) (OutRow :type "/Game/Blueprints/Datas/Struct/ST_WorkSpeed Structure"))
  ; 매프레임 포즈 혹은 움직임 상태에 따라서 워크 스피드 저장
  ;; 무기 들고있나 여부 확인
  (`|ExecutionSequence`
    (:`then_0`
      (set `local.RowName` (`KismetStringLibrary.Conv_BoolToString` (`/Game/Blueprints/Character/BP_Player.bIsWeaponEquipped` (`self.PlayerRef`)))))
    (:`then_1`
      (set `local.RowName` (`KismetStringLibrary.Concat_StrStr` (`local.RowName`) "_" (`|GetEnumeratorNameAsString` (`/Game/Blueprints/Character/BP_Player.CurrentPoseState` (`self.PlayerRef`))))))
    (:`then_2`
      (bind _returnvalue (`|GetDataTableRow` "/Game/Blueprints/Datas/DataTable/DT_WalkSpeeds.DT_WalkSpeeds" (`KismetStringLibrary.Conv_StringToName` (`local.RowName`)))
        (:`then`
          (bind _output_get (set `local.OutRow` _returnvalue))
          (set `self.CachedSpeedData` (select `/Game/Blueprints/Datas/Enum/E_MoveState` (`/Game/Blueprints/Character/BP_Player.CurrentMoveState` (`self.PlayerRef`)) :`NewEnumerator0` (break `/Game/Blueprints/Datas/Struct/ST_WorkSpeed` _output_get) :`NewEnumerator1` (`.Jog_9_72E4434445840241CB85D58DD95177BF` (break `/Game/Blueprints/Datas/Struct/ST_WorkSpeed` _output_get)) :`NewEnumerator2` (`.Run_10_52A82E7D4A1D9560D9F9C68B9D8BD81F` (break `/Game/Blueprints/Datas/Struct/ST_WorkSpeed` _output_get)) :`NewEnumerator3` (`.Aim_11_7B221E5645FCCAF23B1ECCA3E2271FA9` (break `/Game/Blueprints/Datas/Struct/ST_WorkSpeed` _output_get)))))))))

(fn `TryGetPoseTransition`
  (params (TergetPose :type "/Game/Blueprints/Datas/Enum/E_PoseState Enum" :default "NewEnumerator0") (FromPose :type "/Game/Blueprints/Datas/Enum/E_PoseState Enum" :default "NewEnumerator0"))
  (returns (ToPose :type "/Game/Blueprints/Datas/Enum/E_PoseState Enum"))
  (bind _returnvalue (`|GetDataTableRow` "/Game/Blueprints/Datas/DataTable/DT_PoseTransitions.DT_PoseTransitions" (`KismetStringLibrary.Conv_StringToName` (`KismetStringLibrary.Concat_StrStr` (`|GetEnumeratorNameAsString` TergetPose) "_" (`|GetEnumeratorNameAsString` FromPose))))
    (:`then`
      (return (break `/Game/Blueprints/Datas/Struct/ST_PoseTransition` _returnvalue)))
    (:`RowNotFound`
      (`KismetSystemLibrary.PrintString` "못찾음" true true (struct :`G` 0.66 :`B` 1.0 :`A` 1.0) 9999.0))))

(fn `UpdateCameraHeight`
  (params (IsMovingNow :type Boolean))
  (locals (CurrentPose :type String) (RowName :type String))
  (bind _currentposestate (`/Game/Blueprints/Character/BP_Player.CurrentPoseState` (`self.PlayerRef`)))
  (bind (_socketoffset_x _socketoffset_y _socketoffset_z) (`KismetMathLibrary.BreakVector` (`SpringArmComponent.SocketOffset` (`/Game/Blueprints/Character/BP_Player.SpringArm` (`self.PlayerRef`)))))
  (`|ExecutionSequence`
    (:`then_0`
      (set `local.CurrentPose` (`|GetEnumeratorNameAsString` _currentposestate))
      (if (`|EnumInequality` _currentposestate "NewEnumerator1")
        (set `local.RowName` (`local.CurrentPose`))
        (else
          (set `local.RowName` (`local.CurrentPose`))
          (if (`local.IsMovingNow`)
            (set `local.RowName` (`KismetStringLibrary.Concat_StrStr` (`local.CurrentPose`) "_" (`KismetStringLibrary.Conv_BoolToString` (`/Game/Blueprints/Character/BP_Player.bIsWeaponEquipped` (`self.PlayerRef`))) "_Move"))))))
    (:`then_1`
      (bind _returnvalue (`|GetDataTableRow` "/Game/Blueprints/Datas/DataTable/DT_CameraHeight.DT_CameraHeight" (`KismetStringLibrary.Conv_StringToName` (`local.RowName`)))
        (:`then`
          (`self.ChangedCameraHeight` (break `/Game/Blueprints/Datas/Struct/ST_CameraHeight` _returnvalue) _socketoffset_z))))))

(fn `UpdatePitchLimits`
  (params (ToPose :type "/Game/Blueprints/Datas/Enum/E_PoseState Enum" :default "NewEnumerator0"))
  (bind (_returnvalue_roll _returnvalue_pitch) (`KismetMathLibrary.BreakRotator` (`self.GetControlRotation`)))
  (bind (_returnvalue_roll_2 _returnvalue_pitch_2 _returnvalue_yaw) (`KismetMathLibrary.BreakRotator` (`self.GetControlRotation`)))
  (bind (_returnvalue_roll_3 _returnvalue_pitch_3 _returnvalue_yaw_2) (`KismetMathLibrary.BreakRotator` (`self.GetControlRotation`)))
  (`|ExecutionSequence`
    (:`then_0`
      (bind _returnvalue (`|GetDataTableRow` "/Game/Blueprints/Datas/DataTable/DT_PitchLimit.DT_PitchLimit" (`KismetStringLibrary.Conv_StringToName` (`|GetEnumeratorNameAsString` ToPose)))
        (:`then`
          (set `self.CachedTopLimit` (break `/Game/Blueprints/Datas/Struct/ST_PitchLimit` _returnvalue))
          (set `self.CachedBottomLimit` (`.BottomLimit_5_226A038E44690B83409FAD9127327ED3` (break `/Game/Blueprints/Datas/Struct/ST_PitchLimit` _returnvalue))))))
    (:`then_1`
      (if (or (> _returnvalue_pitch (`self.CachedBottomLimit`)) (< _returnvalue_pitch (`self.CachedTopLimit`)))
        _
        (elif (< (`KismetMathLibrary.Abs` (- _returnvalue_pitch (`self.CachedTopLimit`))) (`KismetMathLibrary.Abs` (- _returnvalue_pitch (`self.CachedBottomLimit`))))
          (`self.ChangePitchLimit` (`self.GetControlRotation`) (`KismetMathLibrary.MakeRotator` _returnvalue_roll_2 (`self.CachedTopLimit`) _returnvalue_yaw))
          (else
            (`self.ChangePitchLimit` (`self.GetControlRotation`) (`KismetMathLibrary.MakeRotator` _returnvalue_roll_3 (`self.CachedBottomLimit`) _returnvalue_yaw_2))))))))

(fn `UpdatePose`
  (params (WaitTime :type "Float (double-precision)") (ToPose :type "/Game/Blueprints/Datas/Enum/E_PoseState Enum" :default "NewEnumerator0"))
  (if (!= WaitTime 0.0)
    (set `self.bIsEnableMove` false)
    (`KismetSystemLibrary.K2_SetTimerDelegate` (`|CreateDelegate` :!event `SetEnableMove`) (`local.WaitTime`))
    (`/Game/Blueprints/Character/BP_Player.UpdatePoseState` (`self.PlayerRef`) (`local.ToPose`))
    (else
      (`/Game/Blueprints/Character/BP_Player.UpdatePoseState` (`self.PlayerRef`) (`local.ToPose`)))))

(fn `UpdateWalkSpeed`
  (locals (RowName :type String) (OutRow :type "/Game/Blueprints/Datas/Struct/ST_WorkSpeed Structure"))
  (bind (_cachedspeeddata_forwardspeed _cachedspeeddata_noneforwardspeed) (break `/Game/Blueprints/Datas/Struct/ST_DirectionalSpeed` (`self.CachedSpeedData`)))
  ; WalkSpeed를 저장하는곳
  (`/Game/Blueprints/Character/BP_Player.SetMaxWalkSpeed` (`self.PlayerRef`) (`KismetMathLibrary.SelectFloat` _cachedspeeddata_forwardspeed _cachedspeeddata_noneforwardspeed (`self.IsAcceleratingForwardArc`))))

(fn `UserConstructionScript`)